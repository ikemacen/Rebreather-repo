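; Shark AI pawn that wanders, chases pawns it sees and drains the player's oxygen on contact.
; It roams by chaining AI moves to random navigable points within a short radius of itself, repeating on success.
; Pawn sensing starts a chase, and a retriggerable delay resumes wandering two seconds after the last sighting.
; Capsule overlap with the third-person character subtracts a fixed amount from the HUD oxygen bar's value.
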(event OnComponentBeginOverlap(Capsule)
  (params (OverlappedComponent :type Primitive%20Component%20Object%20Reference) (OtherActor :type Actor%20Object%20Reference) (OtherComp :type Primitive%20Component%20Object%20Reference) (OtherBodyIndex :type Integer) (bFromSweep :type Boolean) (SweepResult :type Hit%20Result%20Structure%20%28by%20ref%29))
  (Utilities|Casting|CastToBP_ThirdPersonCharacter OtherActor)
  (Variables|Default|SetOverlap? true)
  (bind _asbp_gameplay_hud (Utilities|Casting|CastToBP_GameplayHUD (HUD|GetHUD (Game|GetPlayerController 0))))
  (if (Variables|Default|GetOverlap?)
    (Variables|/Game/UI/OxygenBar.OxygenBar_C|SetOxygen (Variables|/Game/UI/BP_GameplayHUD.BP_GameplayHUD_C|GetOxyBarRef _asbp_gameplay_hud) (- (Variables|/Game/UI/OxygenBar.OxygenBar_C|GetOxygen (Variables|/Game/UI/BP_GameplayHUD.BP_GameplayHUD_C|GetOxyBarRef _asbp_gameplay_hud)) 0.1))))

(event OnSeePawn(PawnSensing)
  (params (Pawn :type Pawn%20Object%20Reference))
  (AI|AIMoveTo self "0, 0, 0" Pawn 5.0 false
    (:then
      (Utilities|FlowControl|RetriggerableDelay 2.0)
      (CallFunction|MovetoRandomLocation))))

(event Custom|MoveToRandomLocation
  (bind _randomlocation (Class|NavigationSystemV1|GetRandomLocationinNavigableRadius (Transformation|GetActorLocation) 2e+02 0 "/Script/AIModule.NavFilter_AIControllerDefault"))
  (AI|AIMoveTo self _randomlocation 0 5.0 false
    (:OnSuccess
      (CallFunction|MovetoRandomLocation))))

(event EventBeginPlay
  (CallFunction|MovetoRandomLocation))

(fn ConstructionScript)